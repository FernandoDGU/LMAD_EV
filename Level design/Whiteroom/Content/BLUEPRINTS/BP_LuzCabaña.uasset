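; BP_LuzCabaña is a cabin light that switches on or off as something passes through its ColiLuzCabaña collision volume.
; On begin overlap, the Encendido flag decides whether LuzCabaña is set to a lit intensity or to zero.
; On end overlap, the flag flips, so successive entries alternate the light state.
; Neither event filters the overlapping actor.
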(event `self.ColiLuzCabaña.OnComponentBeginOverlap`
  (params (OverlappedComponent :type "PrimitiveComponent Object Reference") (OtherActor :type "Actor Object Reference") (OtherComp :type "PrimitiveComponent Object Reference") (OtherBodyIndex :type Integer) (bFromSweep :type Boolean) (SweepResult :type "HitResult Structure (by ref)"))
  (if (`self.Encendido`)
    (`LightComponent.SetIntensity` (`self.LuzCabaña`) 1000.0)
    (else
      (`LightComponent.SetIntensity` (`self.LuzCabaña`) 0.0))))

(event `self.ColiLuzCabaña.OnComponentEndOverlap`
  (params (OverlappedComponent :type "PrimitiveComponent Object Reference") (OtherActor :type "Actor Object Reference") (OtherComp :type "PrimitiveComponent Object Reference") (OtherBodyIndex :type Integer))
  (if (`self.Encendido`)
    (set `self.Encendido` false)
    (else
      (set `self.Encendido` true))))

(fn `UserConstructionScript`)