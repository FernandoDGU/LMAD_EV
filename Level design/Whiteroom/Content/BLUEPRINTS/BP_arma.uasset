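; Weapon pickup actor that the player can equip and drop.
; A sphere trigger enables input on the weapon for player controller 0 while overlapped and disables it on exit, without filtering the overlapping actor.
; Equip snaps it to the player character mesh's RightHandSocket and sets TieneArma on ThirdPersonCharacter.
; Unequip clears that flag and detaches the weapon, keeping its world transform.
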(event `self.Sphere.OnComponentBeginOverlap`
  (params (OverlappedComponent :type "PrimitiveComponent Object Reference") (OtherActor :type "Actor Object Reference") (OtherComp :type "PrimitiveComponent Object Reference") (OtherBodyIndex :type Integer) (bFromSweep :type Boolean) (SweepResult :type "HitResult Structure (by ref)"))
  (`self.EnableInput` (`GameplayStatics.GetPlayerControllerFromID` 0)))

(event `self.Sphere.OnComponentEndOverlap`
  (params (OverlappedComponent :type "PrimitiveComponent Object Reference") (OtherActor :type "Actor Object Reference") (OtherComp :type "PrimitiveComponent Object Reference") (OtherBodyIndex :type Integer))
  (`self.DisableInput` (`GameplayStatics.GetPlayerControllerFromID` 0)))

(event `InputAction|Equip`
  (params (Key :type "Key Structure"))
  ;[1 1 1] Equipar arma
  (:`Pressed`
    (`self.Equipar`)))

(event `InputAction|Unequip `
  (params (Key :type "Key Structure"))
  ;[1 1 1] Soltar arma
  (:`Pressed`
    (`self.Soltar`)))

(fn `Equipar`
  (bind _returnvalue (`GameplayStatics.GetPlayerCharacter` 0))
  (`self.K2_AttachToComponent` (`Character.Mesh` _returnvalue) "RightHandSocket" "SnapToTarget" "SnapToTarget" "SnapToTarget")
  (bind _asthird_person_character (cast `/Game/ThirdPersonBP/Blueprints/ThirdPersonCharacter` _returnvalue))
  (set `/Game/ThirdPersonBP/Blueprints/ThirdPersonCharacter.TieneArma?` true _asthird_person_character))

(fn `Soltar`
  (bind _asthird_person_character (cast `/Game/ThirdPersonBP/Blueprints/ThirdPersonCharacter` (`GameplayStatics.GetPlayerCharacter` 0)))
  (set `/Game/ThirdPersonBP/Blueprints/ThirdPersonCharacter.TieneArma?` false _asthird_person_character)
  (`self.K2_DetachFromActor` "KeepWorld" "KeepWorld" "KeepWorld"))

(fn `UserConstructionScript`)